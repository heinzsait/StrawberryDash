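; BP_Crosshair is a crosshair Blueprint whose static mesh spins continuously around its roll axis.
; Each tick advances an Angle variable by delta time at a fixed degrees-per-second rate and writes it to the mesh's relative rotation.
; Once Angle passes a full turn it resets to zero, skipping the rotation update for that frame.
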(event `self.ReceiveTick`
  (params (DeltaSeconds :type "Float (single-precision)"))
  (if (> (`self.angle`) 360.0)
    (set `self.angle` 0.0)
    (else
      (bind _output_get (set `self.angle` (+ (`self.angle`) (* (`GameplayStatics.GetWorldDeltaSeconds`) 60.0))))
      (`SceneComponent.K2_SetRelativeRotation` (`self.StaticMesh`) (`KismetMathLibrary.MakeRotator` _output_get) false false))))

(fn `UserConstructionScript`)